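; Interactable trigger actor that shows an on-screen prompt while the third-person character is in its box and acknowledges a key press.
; Entering the box creates an Interact_Message widget with the configured Words and plays a beep; leaving hides it.
; Tick polls the configured Key during overlap, playing a sound and hiding the prompt through a DoOnce that any begin overlap resets.
; The press triggers no further action here.
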(event `self.ReceiveTick`
  (params (DeltaSeconds :type "Float (single-precision)"))
  (if (`PlayerController.IsInputKeyDown` (`GameplayStatics.GetPlayerController` 0) (`self.Key`))
    (if (`self.IsOverlapping`)
      (`/Engine/EditorBlueprintResources/StandardMacros.DoOnce` false :!label _label
        (:`Completed`
          (`GameplayStatics.PlaySound2D` "/Game/Audio/220212__gameaudio__ping-bing.220212__gameaudio__ping-bing" 1.0 1.0 0.0 null null)
          (`Widget.SetVisibility` (stale `self.Interactable Trigger Box.OnComponentBeginOverlap` _returnvalue) "Hidden" :!label _label_2))))))

(event `self.Interactable Trigger Box.OnComponentBeginOverlap`
  (params (OverlappedComponent :type "PrimitiveComponent Object Reference") (OtherActor :type "Actor Object Reference") (OtherComp :type "PrimitiveComponent Object Reference") (OtherBodyIndex :type Integer) (bFromSweep :type Boolean) (SweepResult :type "HitResult Structure (by ref)"))
  (`|ExecutionSequence`
    (:`then_0`
      (cast `/Game/ThirdPerson/Blueprints/BP_ThirdPersonCharacter` OtherActor)
      (set `self.IsOverlapping` true)
      (bind _returnvalue (`|CreateWidget` "/Game/UI/Interact_Message.Interact_Message_C"))
      (`UserWidget.AddToPlayerScreen` _returnvalue 0)
      (`/Game/UI/Interact_Message.Say New Message` _returnvalue (`self.Words`))
      (`GameplayStatics.PlaySound2D` "/Game/Audio/388046__paep3nguin__beep-up.388046__paep3nguin__beep-up" 1.0 1.0 0.0 null null))
    (:`then_1`
      (goto _label :!via `Reset`))))

(event `self.Interactable Trigger Box.OnComponentEndOverlap`
  (params (OverlappedComponent :type "PrimitiveComponent Object Reference") (OtherActor :type "Actor Object Reference") (OtherComp :type "PrimitiveComponent Object Reference") (OtherBodyIndex :type Integer))
  (cast `/Game/ThirdPerson/Blueprints/BP_ThirdPersonCharacter` OtherActor)
  (set `self.IsOverlapping` false)
  (goto _label_2))

(fn `UserConstructionScript`)
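; Plain road Blueprint that lays spline meshes along an editable spline.
; The construction script loops over each segment between neighboring spline points and adds one of two spline mesh component templates, chosen by the Type variable.
; Each segment takes its start and end from the local locations and tangents of its two points, so the mesh follows the curve.
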(fn `UserConstructionScript`
  (bind _spline (`self.Spline`))
  (for _index (range (+ (- (`SplineComponent.GetNumberOfSplinePoints` (`self.Spline`)) 2) 1))
    (if (== (`self.Type`) 1)
      (bind _returnvalue (`AddComponent|NODE_AddSplineMeshComponent-0`))
      (bind (_location _tangent) (`SplineComponent.GetLocationAndTangentAtSplinePoint` _spline _index "Local"))
      (bind (_location_2 _tangent_2) (`SplineComponent.GetLocationAndTangentAtSplinePoint` _spline (+ _index 1) "Local"))
      (`SplineMeshComponent.SetStartAndEnd` _returnvalue _location _tangent _location_2 _tangent_2 true :!label _label)
      (`SplineMeshComponent.SetStartAndEnd` (stale _returnvalue_2) _location _tangent _location_2 _tangent_2 true)
      (`SceneComponent.K2_AttachToComponent` (stale _returnvalue_2) (`self.DefaultSceneRoot`) "None" "KeepRelative" "KeepRelative" "KeepRelative" true)
      (elif (== (`self.Type`) 2)
        (bind _returnvalue_2 (`AddComponent|NODE_AddSplineMeshComponent-1`))
        (goto _label)))))
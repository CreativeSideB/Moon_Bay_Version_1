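; Industrial ceiling light Blueprint, a placeable fixture that can be set lit or unlit through its On variable.
; The construction script sets the spotlight's visibility from On and swaps material slot 0 on components C1, C2 and C3 between an emissive and an off material.
; The event graph holds only disabled stub events, so the Blueprint has no runtime switching logic of its own.
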(fn `UserConstructionScript`
  (bind _on_ (`self.On?`))
  (bind _emmisive_material (`self.Emmisive Material`))
  (bind _off_material (`self.Off Material`))
  (`SceneComponent.SetVisibility` (`self.SpotLight`) _on_ false)
  (if _on_
    (`|ExecutionSequence`
      (:`then_0`
        (`PrimitiveComponent.SetMaterial` (`self.C1`) 0 _emmisive_material))
      (:`then_1`
        (`PrimitiveComponent.SetMaterial` (`self.C2`) 0 _emmisive_material))
      (:`then_2`
        (`PrimitiveComponent.SetMaterial` (`self.C3`) 0 _emmisive_material)))
    (else
      (`|ExecutionSequence`
        (:`then_0`
          (`PrimitiveComponent.SetMaterial` (`self.C1`) 0 _off_material))
        (:`then_1`
          (`PrimitiveComponent.SetMaterial` (`self.C2`) 0 _off_material))
        (:`then_2`
          (`PrimitiveComponent.SetMaterial` (`self.C3`) 0 _off_material))))))